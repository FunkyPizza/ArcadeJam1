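; Game mode for a small arcade jam game that keeps a level timer of elapsed minutes and seconds.
; BeginPlay zeroes the seconds counter and prints a debug string.
; Tick accumulates delta time into seconds, then increments minutes and resets seconds to zero at each minute mark, dropping any leftover fraction.
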(event EventBeginPlay
  ;[1 1 1] Level Timer
  (Variables|Default|SetLevelSeconds 0.0)
  (Development|PrintString "ArcadeJamGameMode"))

(event EventTick
  (params (DeltaSeconds :type Float%20%28single-precision%29))
  ;[1 1 1] Level Timer
  (bind _output_get (Variables|Default|SetLevelSeconds (+ (Variables|Default|GetLevelSeconds) DeltaSeconds)))
  (if (>= _output_get 6e+01)
    (Math|Float|IncrementFloat (Variables|Default|GetLevelMinutes)
      (:%20%20
        (Variables|Default|SetLevelSeconds 0.0)))))

(fn ConstructionScript)