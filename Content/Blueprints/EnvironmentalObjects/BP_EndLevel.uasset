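; BP_EndLevel is a level exit trigger that advances the player to the next numbered level.
; When a PlayerCharacter overlaps its Box, it plays a win sound and waits six seconds.
; It derives the next level by incrementing the last character of the current level name as a digit.
; Only the first four characters are rejoined and opened, so it assumes four-character names ending in a single digit.
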(event OnComponentBeginOverlap(Box)
  (params (OverlappedComponent :type Primitive%20Component%20Object%20Reference) (OtherActor :type Actor%20Object%20Reference) (OtherComp :type Primitive%20Component%20Object%20Reference) (OtherBodyIndex :type Integer) (bFromSweep :type Boolean) (SweepResult :type Hit%20Result%20Structure%20%28by%20ref%29))
  (Utilities|Casting|CastToPlayerCharacter OtherActor)
  (Audio|PlaySound2D "/Game/Assets/SFX/Win.Win" 1.0 1.0 0.0 0 0)
  (Utilities|FlowControl|Delay 6.0)
  (bind _returnvalue (Game|GetCurrentLevelName true))
  (bind _output_get (Variables|Default|SetNextLevelArray (Utilities|String|GetCharacterArrayfromString _returnvalue)))
  (Utilities|Array|SetArrayElem _output_get (Utilities|Array|LastIndex _output_get) (Utilities|String|ToString(Integer) (+ (Math|Conversions|ToInteger(Byte) (Utilities|Array|Get(acopy) _output_get (Utilities|Array|LastIndex _output_get))) 1)))
  (Game|OpenLevel(byName) (Utilities|String|StringToName (Utilities|String|Append (Utilities|Array|Get(acopy) (Variables|Default|GetNextLevelArray)) (Utilities|Array|Get(acopy) (Variables|Default|GetNextLevelArray) 1) (Utilities|Array|Get(acopy) (Variables|Default|GetNextLevelArray) 2) (Utilities|Array|Get(acopy) (Variables|Default|GetNextLevelArray) 3)))))

(event EventBeginPlay)

(event Collision|EventActorBeginOverlap
  (params (OtherActor :type Actor%20Object%20Reference)))

(event EventTick
  (params (DeltaSeconds :type Float%20%28single-precision%29)))

(fn ConstructionScript)